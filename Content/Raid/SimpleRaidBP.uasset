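; Raid Blueprint for a Twitch chat adventure in which viewers invest caterium and venture from the HUB to a location.
; Preparation shuffles locations, announces three, and listens to BP_Twitch messages for participant votes by name or shorthand.
; After a timed window, the most-voted location wins, participants are shuffled, and one event per participant runs in delayed sequence.
; Completion posts survivors and their caterium to chat.
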(event `self.BeginPreparing`
  (bind _availablelocations (`self.AvailableLocations`))
  (`parent.BeginPreparing`)
  (`|ExecutionSequence`
    (:`then_0`
      (`KismetArrayLibrary.Array_Shuffle` _availablelocations)
      (set `self.Location` (`|GetArrayItem` _availablelocations)))
    (:`then_1`
      (bind _returnvalue (`GameplayStatics.GetActorOfClass` "/Game/Twitch/BP_Twitch.BP_Twitch_C"))
      (add `/Game/Twitch/BP_Twitch.On Message` _returnvalue (`|CreateDelegate` :!event `On Prep Message`)))
    (:`then_2`
      (`KismetSystemLibrary.Delay` 20.0)
      (`self.SendTwitchMessage` (`|FormatText` "The HUB looks close to {loc1}, {loc2}, and {loc3}. Where do you want to go?" (`RaidLocation.Name` (`|GetArrayItem` _availablelocations)) (`RaidLocation.Name` (`|GetArrayItem` _availablelocations 1)) (`RaidLocation.Name` (`|GetArrayItem` _availablelocations 2)))))
    (:`then_3`
      (`KismetSystemLibrary.Delay` 60.0)
      (`self.BeginRaid`))))

(event `self.BeginRaid`
  (bind _outarray (`self.GetParticipants`))
  (`parent.BeginRaid`)
  (`KismetArrayLibrary.Array_Shuffle` _outarray)
  (set `self.NumEvents` (`KismetArrayLibrary.Array_Length` _outarray))
  (bind _returnvalue (`GameplayStatics.GetActorOfClass` "/Game/Twitch/BP_Twitch.BP_Twitch_C"))
  (remove `/Game/Twitch/BP_Twitch.On Message` _returnvalue (`|CreateDelegate` :!event `On Prep Message`))
  (`|ExecutionSequence`
    (:`then_0`
      (bind _result (`self.Calculate Chosen Location`))
      (set `self.Location` _result))
    (:`then_1`
      (`self.SendTwitchMessage` (`|FormatText` "With your {investment} caterium, the group purchases some Paleberries for safety..." (`self.Investment`))))
    (:`then_2`
      (`self.SendTwitchMessage` (`|FormatText` "It's time! Everyone assembles at the HUB and embarks into the {location}..." (`RaidLocation.Name` (`self.Location`)))))
    (:`then_3`
      (`KismetSystemLibrary.Delay` 10.0)
      (`self.RunNextEvent`))))

(event `self.OnRaidEventComplete`
  (`parent.OnRaidEventComplete`)
  (`KismetSystemLibrary.PrintString` (`KismetTextLibrary.Conv_TextToString` (`|FormatText` "Raid Event {num} complete" (`self.Progress`))) true true (struct :`G` 0.66 :`B` 1.0 :`A` 1.0) 20.0)
  (bind _result (`/Engine/EditorBlueprintResources/StandardMacros.IncrementInt` (`self.Progress`))
    (:`  `
      (if (== _result (`self.NumEvents`))
        (`self.Complete`)
        (else
          (`KismetSystemLibrary.Delay` 10.0)
          (`self.RunNextEvent`))))))

(event `self.Complete`
  (`parent.Complete`)
  (`self.CompleteRaid`)
  (`KismetSystemLibrary.PrintString` "Raid Complete" true true (struct :`G` 0.66 :`B` 1.0 :`A` 1.0) 20.0))

(fn `Calculate Chosen Location`
  (returns (Result :type "RaidLocation Object Reference"))
  (locals (Counts :type "Map of RaidLocation Object Reference to Integer") (`Current Max` :type Integer) (`Current Result` :type "RaidLocation Object Reference"))
  (bind _values (`BlueprintMapLibrary.Map_Values` (`self.Votes`)))
  (for _array_element _values
    (bind (_value _returnvalue) (`BlueprintMapLibrary.Map_Find` (`local.Counts`) _array_element))
    (if _returnvalue
      (bind _result (`/Engine/EditorBlueprintResources/StandardMacros.IncrementInt` _value)
        (:`  `
          (if (> _result (`local.Current Max`))
            (set `local.Current Max` _result)
            (set `local.Current Result` _array_element))))
      (else
        (`BlueprintMapLibrary.Map_Add` (`local.Counts`) _array_element 1)
        (if (> 1 (`local.Current Max`))
          (set `local.Current Max` 1)
          (set `local.Current Result` _array_element)))))
  (bind _current_result (`local.Current Result`)
    (:`then`
      (return _current_result))
    (:`else`
      (return (`|GetArrayItem` (`self.AvailableLocations`))))))

(fn `CompleteRaid`
  (locals (TotalInvestment :type Integer))
  (bind _outarray (`self.GetLivingParticipants`))
  (bind _output (`|GetArrayItem` _outarray))
  (switch `int` (`KismetArrayLibrary.Array_Length` _outarray)
    (:`Default`
      (for _array_element _outarray
        (`KismetArrayLibrary.Array_Add` (`self.SurvivorsAndWinnings`) (`KismetTextLibrary.Conv_TextToString` (`|FormatText` "{name} ({winnings})" (`RaidParticipantComponent.GetName` _array_element) (+ (`RaidParticipantComponent.Winnings` _array_element) (`RaidParticipantComponent.Investment` _array_element))))))
      (`self.SendTwitchMessage` (`|FormatText` "The adventure is complete! Survivors: {survivors}" (`KismetStringLibrary.JoinStringArray` (`self.SurvivorsAndWinnings`) ", "))))
    (:`0`
      (`self.SendTwitchMessage` "The adventure is complete, but nobody survived :( All the caterium is lost"))
    (:`1`
      (`self.SendTwitchMessage` (`|FormatText` "The adventure is complete! Only {survivor} survived. They get all the {amount} caterium found..." (`RaidParticipantComponent.GetName` _output) (`RaidParticipantComponent.Winnings` _output))))))

(fn `GetActiveParticipant`
  (returns (ReturnValue :type "RaidParticipantComponent Object Reference"))
  (if (`self.IsInProgress`)
    (return (`self.GetParticipant` (`self.Progress`)))))

(fn `On Prep Message`
  (params (Author :type "TwitchMessageAuthor Structure") (Message :type String))
  (locals (Messager :type "RaidParticipantComponent Object Reference"))
  (for _array_element (`self.GetParticipants`)
    (if (== (`RaidParticipantComponent.GetName` _array_element) Author_Name)
      (set `local.Messager` _array_element)
      (break)))
  (`local.Messager`
    (:`then`
      (for (_array_element_2 _array_index) (`self.AvailableLocations`)
        (`|ExecutionSequence`
          (:`then_0`
            (if (`KismetStringLibrary.Contains` (`local.Message`) (`KismetTextLibrary.Conv_TextToString` (`RaidLocation.Name` _array_element_2)))
              (`BlueprintMapLibrary.Map_Add` (`self.Votes`) (`local.Messager`) _array_element_2)
              (return)
              (else
                (for _array_element_3 (`RaidLocation.AcceptedShorthands` _array_element_2)
                  (if (`KismetStringLibrary.Contains` (`local.Message`) _array_element_3)
                    (`BlueprintMapLibrary.Map_Add` (`self.Votes`) (`local.Messager`) _array_element_2)
                    (return))))))
          (:`then_1`
            (if (> _array_index 2)
              (return))))))
    (:`else`)))

(fn `On Preparing Message1`)

(fn `UserConstructionScript`)
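; Test raid Blueprint for a Twitch chat adventure in which participants risk and win caterium.
; After a short preparation delay it shuffles participants and runs one event per participant, tracking the active one by progress index.
; Before each event, living players enter the stage and dead ones are hidden.
; On completion it reports survivors and winnings to Twitch chat, with separate messages for none, one or several survivors.
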(event `self.BeginPreparing`
  (`parent.BeginPreparing`)
  (`KismetSystemLibrary.Delay` 2.0)
  (`self.BeginRaid`))

(event `self.BeginRaid`
  (bind _outarray (`self.GetParticipants`))
  (`parent.BeginRaid`)
  (`KismetArrayLibrary.Array_Shuffle` _outarray)
  (set `self.NumEvents` (`KismetArrayLibrary.Array_Length` _outarray))
  (`GameplayStatics.GetActorOfClass` "/Game/Twitch/BP_Twitch.BP_Twitch_C")
  (`self.SendTwitchMessage` "Test raid Beginning!")
  (`KismetSystemLibrary.Delay` 0.016 :!label _label)
  (`self.Setup Player Positions`)
  (`self.RunNextEvent`))

(event `self.OnRaidEventComplete`
  (`parent.OnRaidEventComplete`)
  (bind _result (`/Engine/EditorBlueprintResources/StandardMacros.IncrementInt` (`self.Progress`))
    (:`  `
      (if (== _result (`self.NumEvents`))
        (`self.Complete`)
        (else
          (goto _label))))))

(event `self.Complete`
  (`parent.Complete`)
  (`self.CompleteRaid`)
  (`KismetSystemLibrary.PrintString` "Raid Complete" true true (struct :`G` 0.66 :`B` 1.0 :`A` 1.0) 20.0))

(fn `CompleteRaid`
  (locals (TotalInvestment :type Integer))
  (bind _outarray (`self.GetLivingParticipants`))
  (bind _output (`|GetArrayItem` _outarray))
  (switch `int` (`KismetArrayLibrary.Array_Length` _outarray)
    (:`Default`
      (for _array_element _outarray
        (`KismetArrayLibrary.Array_Add` (`self.SurvivorsAndWinnings`) (`KismetTextLibrary.Conv_TextToString` (`|FormatText` "{name} ({winnings})" (`RaidParticipantComponent.GetName` _array_element) (+ (`RaidParticipantComponent.Winnings` _array_element) (`RaidParticipantComponent.Investment` _array_element))))))
      (`self.SendTwitchMessage` (`|FormatText` "The adventure is complete! Survivors: {survivors}" (`KismetStringLibrary.JoinStringArray` (`self.SurvivorsAndWinnings`) ", "))))
    (:`0`
      (`self.SendTwitchMessage` "The adventure is complete, but nobody survived :( All the caterium is lost"))
    (:`1`
      (`self.SendTwitchMessage` (`|FormatText` "The adventure is complete! Only {survivor} survived. They get all the {amount} caterium found..." (`RaidParticipantComponent.GetName` _output) (`RaidParticipantComponent.Winnings` _output))))))

(fn `GetActiveParticipant`
  (returns (ReturnValue :type "RaidParticipantComponent Object Reference"))
  (if (`self.IsInProgress`)
    (return (`self.GetParticipant` (`self.Progress`)))))

(fn `Setup Player Positions`
  (for _array_element (`self.GetParticipants`)
    (if (`RaidParticipantComponent.IsAlive` _array_element)
      (bind _returnvalue (`ActorComponent.GetOwner` _array_element))
      (bind _aschat_player_bp (cast `/Game/Characters/ChatPlayerBP` _returnvalue))
      (`/Game/Characters/ChatPlayerBP.Enter Stage` _aschat_player_bp)
      (else
        (`self.SetActorHiddenInGame` _returnvalue true)))))

(fn `UserConstructionScript`)
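; BP_CircleHoverComponent is an actor component in the MercerSacrifice raid event folder that makes its owner drift in a small looping hover.
; BeginPlay randomizes starting angle, speed and spin direction, so instances move out of sync.
; Tick advances the angle and adds sine and cosine local X/Z offsets to the owner each frame, so loop size depends on frame rate.
; An unused branch offsets only the Paper sprite component instead.
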(event `self.ReceiveBeginPlay`
  (set `self.Speed` (* (`KismetMathLibrary.RandomFloatInRange` 2.0 3.0) (`KismetMathLibrary.SelectInt` 1 -1 (`KismetMathLibrary.RandomBool`))))
  (set `self.Angle` (`KismetMathLibrary.RandomFloatInRange` 0.0 360.0)))

(event `self.ReceiveTick`
  (params (DeltaSeconds :type "Float (single-precision)"))
  (bind _output_get (set `self.Angle` (+ (* DeltaSeconds (`self.Speed`)) (`self.Angle`))))
  (`Actor.K2_AddActorLocalOffset` (`self.GetOwner`) (`KismetMathLibrary.MakeVector` (* (`KismetMathLibrary.Sin` _output_get) 0.15) 0.0 (* (`KismetMathLibrary.Cos` _output_get) 0.1)) false false))
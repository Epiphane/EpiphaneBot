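; Twitch integration actor that connects the streamer's channel to the raid and Caterium economy game.
; On BeginPlay it authenticates with saved credentials, falling back to local login, then connects chat and channel-point events.
; Chat commands let viewers join raids with Caterium investments, gift currency, check balances and trophies, and set avatars.
; Channel-point redemptions grant Caterium by parsing the reward title, while raid cooldown and prestige events post chat announcements.
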(event `self.ReceiveBeginPlay`
  (bind _returnvalue (`GameplayStatics.LoadGameFromSlot` (`self.Credential Slot Name`)))
  (`/Engine/EditorBlueprintResources/StandardMacros.IsValid` _returnvalue
    (:`Is Valid`
      (bind _asbp_save_game (cast `/Game/Twitch/BP_SaveGame` _returnvalue)
        (:`then`
          (`TwitchPluginBPLibrary.SetChatOutputEnabled` (`/Game/Twitch/BP_SaveGame.Chat Output Enabled` _asbp_save_game))
          (`self.TryAuth` (`/Game/Twitch/BP_SaveGame.Credentials` _asbp_save_game) true))
        (:`CastFailed`
          (`self.DoLogin` :!label _label))))
    (:`Is Not Valid`
      (goto _label))))

(event `TryAuth`
  (params (Credentials :type "TwitchLoginCredentials Structure") (FallbackToLogin :type Boolean))
  (bind (_oauthtoken _username) (break `TwitchLoginCredentials` Credentials))
  (bind _returnvalue (subsystem `TwitchEventsSubsystem`))
  (bind (_twitchuser _twitchchat) (`TwitchChatConnector.RequestFeed` (`|CreateDelegate` :!event `OnTwitchMessage`) (`|CreateDelegate` :!event `HandleCheer`) Credentials _username)
    (:`OnSuccessfulLogin`
      (`|ExecutionSequence`
        (:`then_0`
          (`self.SetupCommands` _twitchchat)
          (bind _output_get (set `self.Twitch Chat` _twitchchat))
          (bind _output_get_2 (set `RaidManager.Chat` _output_get (subsystem `RaidManager`)))
          (`KismetSystemLibrary.PrintString` "Connection Succeeded")
          (add `RaidManager.OnRaidCooldownOver` (subsystem `RaidManager`) (delegate `On Raid Cooldown Over`)))
        (:`then_1`
          (`TwitchEventsSubsystem.OpenConnection` _returnvalue Credentials)
          (add `TwitchEventsSubsystem.OnChannelPointRedemption` _returnvalue (`|CreateDelegate` :!event `On Channel Point Redemption`)))
        (:`then_2`
          (`self.On Channel Login` _username))
        (:`then_3`
          (add `EpiUserDataSubsystem.PrestigeChangedEvent` (subsystem `EpiUserDataSubsystem`) (delegate `On Prestige changed`)))))
    (:`OnFailedLogin`
      (if FallbackToLogin
        (`self.DoLogin`)
        (else
          (`KismetSystemLibrary.PrintString` "Connection Failed")
          (`GameplayStatics.DeleteGameInSlot` (`self.Credential Slot Name`)))))))

(event `On Raid Cooldown Over`
  (`TwitchPluginBPLibrary.SendTwitchMessage` (stale `TryAuth` _output_get_2) "CooldownOverMessage"))

(event `DoLogin`
  (bind _credentials (`LocalTwitchLoginTask.PerformLocalTwitchLogin`)
    (:`OnSuccess`
      (`self.SaveLocalCredentials` _credentials)
      (`self.TryAuth` _credentials))
    (:`OnFail`
      (`KismetSystemLibrary.PrintString` "Login Failed"))))

(event `On Prestige changed`
  (params (ID :type Integer) (NewValue :type Integer))
  (bind _returnvalue (`EpiUserDataSubsystem.GetNameForId` (subsystem `EpiUserDataSubsystem`) ID))
  (switch `int` NewValue
    (:`Default`
      (`TwitchPluginBPLibrary.SendTwitchMessage` (`self.Twitch Chat`) (`|FormatText` "{participant} has earned 2 billion caterium and earned a golden nut trophy, for a total of {user.Prestige} trophies! Congratulations epiphaLuck1" _returnvalue NewValue)))
    (:`1`
      (`TwitchPluginBPLibrary.SendTwitchMessage` (`self.Twitch Chat`) (`|FormatText` "{participant} has earned 2 billion caterium and earned their first golden nut trophy! Congratulations epiphaLuck1" _returnvalue)))))

(event `Clear Authentication`
  (`self.DoLogin`))

(fn `Get Caterium Command`
  (params (Parameters :type "Array of String (by ref)") (Sender :type "TwitchMessageAuthor Structure"))
  (bind _returnvalue (`SimpleEpiUser.GetUserFromAuthor` Sender))
  (`TwitchPluginBPLibrary.SendTwitchMessage` (`self.Twitch Chat`) (`|FormatText` "{user}, you have {user.Caterium} caterium!" (`EpiUser.GetUserName` _returnvalue) (`EpiUser.GetCaterium` _returnvalue)))
  (return))

(fn `Get Nuts`
  (params (Parameters :type "Array of String (by ref)") (Sender :type "TwitchMessageAuthor Structure"))
  (bind _returnvalue (`SimpleEpiUser.GetUserFromAuthor` Sender))
  (bind _returnvalue_2 (`EpiUser.GetPrestige` _returnvalue))
  (switch `int` _returnvalue_2
    (:`Default`
      (bind _returnvalue_3 (`EpiUser.GetUserName` _returnvalue))
      (`TwitchPluginBPLibrary.SendTwitchMessage` (`self.Twitch Chat`) (`|FormatText` "{user}, you have {user.Prestige} golden nut trophies! epiphaLuck2" _returnvalue_3 _returnvalue_2)))
    (:`0`
      (`TwitchPluginBPLibrary.SendTwitchMessage` (`self.Twitch Chat`) (`|FormatText` "{user}, you have {user.Prestige} golden nut trophies! epiphaPro2" _returnvalue_3 _returnvalue_2)))
    (:`1`
      (`TwitchPluginBPLibrary.SendTwitchMessage` (`self.Twitch Chat`) (`|FormatText` "{user}, you have {user.Prestige} golden nut trophy! epiphaLuck2" _returnvalue_3 _returnvalue_2)))))

(fn `HandleCheer`
  (params (TwitchCheer :type "TwitchCheer Structure")))

(fn `On Channel Point Redemption`
  (params (Redeem :type "ChannelPointAPIRedemption Structure") (UserId :type String) (UserName :type String))
  (bind (_id _title) (break `ChannelPointAPIRedemption` Redeem))
  (if (`KismetStringLibrary.MatchesWildcard` _title "Buy * Caterium")
    (bind _returnvalue (`SimpleEpiUser.Get` UserName (`KismetStringLibrary.Conv_StringToInt64` UserId)))
    (`ChatPlayer.AddCaterium` _returnvalue (`KismetStringLibrary.Conv_StringToInt` (`KismetStringLibrary.GetSubstring` _title 4 10)))
    (`TwitchPluginBPLibrary.SendTwitchMessage` (`self.Twitch Chat`) (`|FormatText` "{player}, you now have {caterium} caterium!" (`EpiUser.GetUserName` _returnvalue) (`EpiUser.GetCaterium` _returnvalue)))))

(fn `OnGiveMessage`
  (params (Parameters :type "Array of String") (Sender :type "TwitchMessageAuthor Structure"))
  (locals (User :type "EpiUser Interface"))
  (bind _output (`|GetArrayItem` Parameters))
  (bind _output_2 (`|GetArrayItem` Parameters 1))
  (bind _user (`local.User`))
  (bind _returnvalue (`EpiUser.GetCaterium` (`local.User`)))
  (bind _returnvalue_2 (`KismetStringLibrary.Conv_StringToInt` _output_2))
  (if (>= (`KismetArrayLibrary.Array_Length` Parameters) 2)
    (bind _returnvalue_3 (`SimpleEpiUser.GetUserFromAuthor` Sender))
    (set `local.User` _returnvalue_3)
    (bind _returnvalue_4 (`SimpleEpiUser.GetUserFromName` _output))
    (`/Engine/EditorBlueprintResources/StandardMacros.IsValid` _returnvalue_4
      (:`Is Valid`
        ;[1 1 1] Have enough Caterium?
        (if (>= _returnvalue _returnvalue_2)
          ;[1 1 1] Input Validation
          (if (>= _returnvalue_2 0)
            (`ChatPlayer.GiveCaterium` _user _returnvalue_4 _returnvalue_2)
            (`TwitchPluginBPLibrary.SendTwitchMessage` (`self.Twitch Chat`) (`|FormatText` "{sender} gives {recipient} {amount} Caterium!" (`EpiUser.GetUserName` _user) (`EpiUser.GetUserName` _returnvalue_4) _returnvalue_2))
            (else
              (`TwitchPluginBPLibrary.SendTwitchMessage` (`self.Twitch Chat`) (`|FormatText` "Invalid amount: {input}" _output_2))))
          (else
            (`TwitchPluginBPLibrary.SendTwitchMessage` (`self.Twitch Chat`) (`|FormatText` "NotEnoughCateriumMessage" _returnvalue)))))
      (:`Is Not Valid`
        (`TwitchPluginBPLibrary.SendTwitchMessage` (`self.Twitch Chat`) (`|FormatText` "I couldn't find {name} :( Perhaps they haven't participated in a raid yet?" _output))))
    (else
      (`TwitchPluginBPLibrary.SendTwitchMessage` (`self.Twitch Chat`) "Usage: !give <person> <amount>"))))

(fn `OnRaidMessage`
  (params (Parameters :type "Array of String") (Sender :type "TwitchMessageAuthor Structure"))
  (locals (Investment :type Integer) (User :type "EpiUser Interface"))
  (bind ((`Color` _color) (`Name` _name) (`UserId` _userid)) (break `TwitchMessageAuthor` Sender))
  (bind _returnvalue (`KismetMathLibrary.RandomFloatInRange` -300.0 300.0))
  (bind _output (`|GetArrayItem` Parameters))
  (bind _investment (`local.Investment`))
  (bind _investment_2 (`local.Investment`))
  (bind (_b _g _r _a) (break `Color` _color))
  (bind _returnvalue_2 (`EpiUser.GetCaterium` (`local.User`)))
  (if (>= (`KismetArrayLibrary.Array_Length` Parameters) 1)
    (bind _returnvalue_3 (`SimpleEpiUser.Get` _name (`KismetStringLibrary.Conv_StringToInt64` _userid) (make `LinearColor` (/ _r 255.0) (/ _g 255.0) (/ _b 255.0) (/ _a 255.0))))
    (set `local.User` _returnvalue_3)
    ;[1 1 1] Handle "all"
    (if (== _output "all")
      (set `local.Investment` (`EpiUser.GetCaterium` (`local.User`)))
      (else
        (set `local.Investment` (`KismetStringLibrary.Conv_StringToInt` _output))))
    ;[1 1 1] Have enough Caterium?
    (if (>= _returnvalue_2 (`local.Investment`))
      ;[1 1 1] Input Validation
      (if (>= (`local.Investment`) 1)
        (bind (_currentraid _participant _cooldown) (`RaidManager.GetRaidEligibility` (subsystem `RaidManager`) (`local.User`))
          (:`NoCurrentRaid`
            ;[1 1 1] New Raid!
            (bind _returnvalue_4 (`RaidManager.StartRaid` (subsystem `RaidManager`) (`self.Raid Class`)))
            (bind _returnvalue_5 (`Raid.Join` _returnvalue_4 (`local.User`) "/Game/Characters/ChatPlayerBP.ChatPlayerBP_C" (`local.Investment`)))
            (`self.K2_AddActorWorldOffset` _returnvalue_5 (`KismetMathLibrary.MakeVector` _returnvalue) false false)
            (`TwitchPluginBPLibrary.SendTwitchMessage` (`self.Twitch Chat`) (`|FormatText` "CreationMessage" (`EpiUser.GetUserName` (`local.User`)))))
          (:`RaidIsJoinable`
            ;[1 1 1] Join Raid
            (bind _returnvalue_6 (`Raid.Join` _currentraid (`local.User`) "/Game/Characters/ChatPlayerBP.ChatPlayerBP_C" _investment_2))
            (`self.K2_AddActorWorldOffset` _returnvalue_6 (`KismetMathLibrary.MakeVector` _returnvalue) false false)
            (`TwitchPluginBPLibrary.SendTwitchMessage` (`self.Twitch Chat`) (`|FormatText` "UserJoinMessage" (`EpiUser.GetUserName` (`local.User`)) _investment_2)))
          (:`AlreadyParticipating`
            ;[1 1 1] Change Investment
            (set `RaidParticipantComponent.Investment` _investment _participant)
            (`TwitchPluginBPLibrary.SendTwitchMessage` (`self.Twitch Chat`) (`|FormatText` "NewInvestmentMessage" (`RaidParticipantComponent.GetName` _participant) _investment)))
          (:`RaidIsOngoing`
            ;[1 1 1] Already Running :(
            (`TwitchPluginBPLibrary.SendTwitchMessage` (`self.Twitch Chat`) (`|FormatText` "AlreadyRunningMessage")))
          (:`Cooldown`
            (bind (_days _hours _minutes _seconds) (`KismetMathLibrary.BreakTimespan` (`KismetMathLibrary.MakeTimespan` 0 0 0 (`KismetMathLibrary.FTrunc` _cooldown))))
            ;[1 1 1] Cooldown
            (if (> _minutes 0)
              (if (>= _seconds 10)
                (`TwitchPluginBPLibrary.SendTwitchMessage` (`self.Twitch Chat`) (`|FormatText` "CooldownMessage" (`|FormatText` "{minutes}:{seconds}" _minutes _seconds)))
                (else
                  (`TwitchPluginBPLibrary.SendTwitchMessage` (`self.Twitch Chat`) (`|FormatText` "CooldownMessage" (`|FormatText` "{minutes}:0{seconds}" _minutes _seconds)))))
              (else
                (`TwitchPluginBPLibrary.SendTwitchMessage` (`self.Twitch Chat`) (`|FormatText` "CooldownMessage" (`|FormatText` "{seconds}s" _seconds)))))))
        (else
          (`TwitchPluginBPLibrary.SendTwitchMessage` (`self.Twitch Chat`) (`|FormatText` "InvalidInvestmentMessage"))))
      (else
        (`TwitchPluginBPLibrary.SendTwitchMessage` (`self.Twitch Chat`) (`|FormatText` "NotEnoughCateriumMessage" _returnvalue_2))))
    (else
      (`TwitchPluginBPLibrary.SendTwitchMessage` (`self.Twitch Chat`) "RaidUsage"))))

(fn `OnTwitchMessage`
  (params (Message :type "TwitchMessage Structure"))
  (bind (_author _messagebody) (break `TwitchMessage` Message))
  (`self.On Message` _author _messagebody))

(fn `SaveLocalCredentials`
  (params (Credentials :type "TwitchLoginCredentials Structure"))
  (bind _returnvalue (`GameplayStatics.CreateSaveGameObject` "/Game/Twitch/BP_SaveGame.BP_SaveGame_C"))
  (set `/Game/Twitch/BP_SaveGame.Credentials` Credentials _returnvalue)
  (set `/Game/Twitch/BP_SaveGame.Chat Output Enabled` (`TwitchPluginBPLibrary.GetChatOutputEnabled`) _returnvalue)
  (`GameplayStatics.SaveGameToSlot` _returnvalue (`self.Credential Slot Name`)))

(fn `Set Avatar`
  (params (Parameters :type "Array of String (by ref)") (Sender :type "TwitchMessageAuthor Structure"))
  (if (>= (`KismetArrayLibrary.Array_Length` Parameters) 1)
    (bind _returnvalue (`|GetDataTableRow` "/Game/Characters/Avatars/AvailableAvatars.AvailableAvatars" (`KismetStringLibrary.Conv_StringToName` (`|GetArrayItem` Parameters)))
      (:`then`
        (bind _returnvalue_2 (`SimpleEpiUser.GetUserFromAuthor` (`local.Sender`)))
        (`EpiUser.SetAvatar` _returnvalue_2 (`.Asset_2_7B548C034265D6F16BD0E8AEC60D9C62` (break `/Game/Characters/Avatars/AvatarDataEntry` _returnvalue)))
        (return)))
    (else
      (`TwitchPluginBPLibrary.SendTwitchMessage` (`self.Twitch Chat`) "Usage: !avatar <name>"))))

(fn `SetupCommands`
  (params (Chat :type "TwitchChatConnector Object Reference"))
  (`TwitchPluginBPLibrary.CreateTwitchCommand` Chat "raid" "Go on an adventure!" "RaidUsage" 1 true (`|CreateDelegate` :!event `OnRaidMessage`))
  (`TwitchPluginBPLibrary.CreateTwitchCommand` Chat "give" "Give someone else Caterium" "!give <person> <amount>" 2 true (`|CreateDelegate` :!event `OnGiveMessage`))
  (`TwitchPluginBPLibrary.CreateTwitchCommand` Chat "gift" "Give someone else Caterium" "!give <person> <amount>" 2 true (`|CreateDelegate` :!event `OnGiveMessage`))
  (`TwitchPluginBPLibrary.CreateTwitchCommand` Chat "caterium" "See how much caterium you have" "!caterium" 0 true (`|CreateDelegate` :!event `Get Caterium Command`))
  (`TwitchPluginBPLibrary.CreateTwitchCommand` Chat "gold" "See how much caterium you have" "!gold" 0 true (`|CreateDelegate` :!event `Get Caterium Command`))
  (`TwitchPluginBPLibrary.CreateTwitchCommand` Chat "nuts" "See how many golden nuts you have" "!nuts" 0 true (`|CreateDelegate` :!event `Get Nuts`))
  (`TwitchPluginBPLibrary.CreateTwitchCommand` Chat "avatar" "Set your avatar" "!avatar <name>" 1 true (`|CreateDelegate` :!event `Set Avatar`)))

(fn `UserConstructionScript`)
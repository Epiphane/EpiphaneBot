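; ChatPlayerBP is a character representing a named chat user, with a floating text label in that user's color.
; On BeginPlay it fills the TextRender with the user name and color and nudges its height by a random amount.
; EnterStage rebuilds the InterpToMovement path from two randomized X-axis points with a random duration and restarts it, sliding the character onto the stage.
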(event `self.ReceiveBeginPlay`
  (bind (_returnvalue_r _returnvalue_g _returnvalue_b _returnvalue_a) (break `LinearColor` (`EpiUser.GetUserColor`)))
  (bind _textrender (`self.TextRender`))
  (`TextRenderComponent.K2_SetText` (`self.TextRender`) (`KismetTextLibrary.Conv_StringToText` (`EpiUser.GetUserName`)))
  (`TextRenderComponent.SetTextRenderColor` _textrender (`KismetMathLibrary.Conv_LinearColorToColor` (`EpiUser.GetUserColor`)))
  (`SceneComponent.K2_AddRelativeLocation` _textrender (`KismetMathLibrary.MakeVector` 0.0 0.0 (`KismetMathLibrary.RandomFloatInRange` -7.0 6.0)) false false)
  (`TextRenderComponent.SetTextRenderColor` (`self.TextRender`) (make `Color` (`KismetMathLibrary.Conv_IntToByte` (`KismetMathLibrary.FFloor` (* _returnvalue_b 255.0))) (`KismetMathLibrary.Conv_IntToByte` (`KismetMathLibrary.FFloor` (* _returnvalue_g 255.0))) (`KismetMathLibrary.Conv_IntToByte` (`KismetMathLibrary.FFloor` (* _returnvalue_r 255.0))) (`KismetMathLibrary.Conv_IntToByte` (`KismetMathLibrary.FFloor` (* _returnvalue_a 255.0))))))

(fn `Enter Stage`
  (bind _movement (`self.Movement`))
  (set `InterpToMovementComponent.Duration` (`KismetMathLibrary.RandomFloatInRange` 1.0 1.5) _movement)
  (`InterpToMovementComponent.ResetControlPoints` _movement)
  (set `InterpToMovementComponent.ControlPoints` (`|MakeArray` (make `InterpControlPoint` (`KismetMathLibrary.MakeVector` (`KismetMathLibrary.RandomFloatInRange` -550.0 -500.0)) false) (make `InterpControlPoint` (`KismetMathLibrary.MakeVector` (`KismetMathLibrary.RandomFloatInRange` -324.0 -204.0)) false) :!type "InterpControlPoint Structure") _movement)
  (`InterpToMovementComponent.FinaliseControlPoints` _movement)
  (`InterpToMovementComponent.RestartMovement` _movement 1.0))

(fn `UserConstructionScript`)
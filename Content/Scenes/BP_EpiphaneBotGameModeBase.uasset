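; Game mode that auto-starts a debug raid for the current level when no BP_Twitch actor already exists.
; On BeginPlay it spawns BP_Twitch and waits for channel login, then searches the SimpleRaidEvents table for an event whose level matches the loaded one.
; On a match, it starts a TestRaidBP, joins DebugUsers at random X offsets, assigns the event class and begins the raid.
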(event `self.ReceiveBeginPlay`
  (bind _returnvalue (`GameplayStatics.GetActorOfClass` "/Game/Twitch/BP_Twitch.BP_Twitch_C"))
  (`/Engine/EditorBlueprintResources/StandardMacros.IsValid` _returnvalue
    (:`Is Not Valid`
      (`|ExecutionSequence`
        (:`then_0`
          (bind _returnvalue_2 (`|SpawnActorFromClass` "/Game/Twitch/BP_Twitch.BP_Twitch_C" (`KismetMathLibrary.MakeTransform` (0.0 0.0 0.0)) "Undefined" "MultiplyWithRoot" null "/Game/Raid/TestRaidBP.TestRaidBP_C" null))
          (add `/Game/Twitch/BP_Twitch.On Channel Login` _returnvalue_2 (delegate `On Login`)))))))

(event `On Login`
  (params (`Channel Name` :type String))
  (bind (_event_class _success) (`self.FindEventForLevel`))
  (if _success
    (`|ExecutionSequence`
      (:`then_0`
        (bind _returnvalue (`RaidManager.StartRaid` (subsystem `RaidManager`) "/Game/Raid/TestRaidBP.TestRaidBP_C"))
        (for _array_element (`self.Debug_Users`)
          (bind _returnvalue_2 (`SimpleEpiUser.GetUserFromAuthor` _array_element))
          (bind _returnvalue_3 (`Raid.Join` _returnvalue _returnvalue_2 "/Game/Characters/ChatPlayerBP.ChatPlayerBP_C" 10))
          (`self.K2_AddActorWorldOffset` _returnvalue_3 (`KismetMathLibrary.MakeVector` (`KismetMathLibrary.RandomFloatInRange` -300.0 300.0)) false false)))
      (:`then_1`
        (bind _astest_raid_bp (cast `/Game/Raid/TestRaidBP` _returnvalue))
        (set `/Game/Raid/TestRaidBP.Event Class` (break `RaidEventRowStruct` _event_class) _astest_raid_bp)
        (`Raid.BeginRaid` _astest_raid_bp)))))

(fn `FindEventForLevel`
  (returns (`Event Class` :type "RaidEventRowStruct Structure") (Success :type Boolean))
  (bind _outrownames (`DataTableFunctionLibrary.GetDataTableRowNames` "/Game/Raid/Events/SimpleRaidEvents.SimpleRaidEvents"))
  (for _array_element _outrownames
    (bind _returnvalue (`|GetDataTableRow` "/Game/Raid/Events/SimpleRaidEvents.SimpleRaidEvents" _array_element)
      (:`then`
        (bind _asevent_with_level (castclass `/Game/Raid/Events/EventWithLevel` (`.EventClass` (break `RaidEventRowStruct` _returnvalue))))
        (bind _returnvalue_2 (`GameplayStatics.GetCurrentLevelName` true))
        (if (== _returnvalue_2 (`.RightS` (`KismetStringLibrary.Split` (`KismetSystemLibrary.Conv_SoftObjectReferenceToString` (defaults `Object` _asevent_with_level)) ".")))
          (return _returnvalue true)))))
  (return (struct) false))

(fn `UserConstructionScript`)
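; CrabBP is a decorative 2D crab creature that sways continuously in a small elliptical loop.
; BeginPlay randomizes the starting phase angle so separate instances can move out of sync.
; Tick advances the angle by delta time and adds sine and cosine local offsets to the PaperSprite on X and Z.
; The offsets are not scaled by delta time, so the loop's size depends on frame rate.
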(event `self.ReceiveBeginPlay`
  (set `self.Angle` (`KismetMathLibrary.RandomFloatInRange` 0.0 3.14)))

(event `self.ReceiveTick`
  (params (DeltaSeconds :type "Float (single-precision)"))
  (bind _output_get (set `self.Angle` (+ (* DeltaSeconds 2.0) (`self.Angle`))))
  (`SceneComponent.K2_AddLocalOffset` (`self.PaperSprite`) (`KismetMathLibrary.MakeVector` (* (`KismetMathLibrary.Sin` _output_get) 0.15) 0.0 (* (`KismetMathLibrary.Cos` _output_get) 0.1)) false false))

(fn `UserConstructionScript`)